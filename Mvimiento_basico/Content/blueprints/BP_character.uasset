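; Player character Blueprint with Enhanced Input movement, camera look, jumping, a timed speed boost, a dash and a target lock.
; Boost temporarily raises walk speed and dash launches along current velocity, each gated by a DoOnce reset on input completion, after a delay for boost.
; Tab toggles the lock: a camera-direction sphere trace stores a pawn, and Tick turns control rotation toward it until cleared.
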(event Input|EnhancedActionEvents|EnhancedInputActionIA_mover
  (params (ActionValue :type Vector%202D%20Structure) (ElapsedSeconds :type Float%20%28double-precision%29) (TriggeredSeconds :type Float%20%28double-precision%29) (InputAction :type Input%20Action%20Object%20Reference :default "/Game/Inputs/IA_mover.IA_mover"))
  (bind _returnvalue (Pawn|GetControlRotation :!class /Script/Engine.Pawn))
  ;[0.15 0.15 0.15 0.5] Movimientos basicos
  (Pawn|Input|AddMovementInput (Math|Vector|GetRightVector (Math|Rotator|MakeRotator (.roll _returnvalue) 0.0 (.yaw _returnvalue))) (.x ActionValue) false)
  (Pawn|Input|AddMovementInput (Math|Vector|GetForwardVector (Math|Rotator|MakeRotator 0.0 0.0 (.yaw (Pawn|GetControlRotation :!class /Script/Engine.Pawn)))) (.y ActionValue) false))

(event Input|EnhancedActionEvents|EnhancedInputActionIA_Saltar
  (params (ActionValue :type Boolean) (ElapsedSeconds :type Float%20%28double-precision%29) (TriggeredSeconds :type Float%20%28double-precision%29) (InputAction :type Input%20Action%20Object%20Reference :default "/Game/Inputs/IA_Saltar.IA_Saltar"))
  ;[0.15 0.15 0.15 0.5] Saltar
  (:Started
    (Character|Jump))
  (:Completed
    (Character|StopJumping)))

(event Input|EnhancedActionEvents|EnhancedInputActionIA_Mirar
  (params (ActionValue :type Vector%202D%20Structure) (ElapsedSeconds :type Float%20%28double-precision%29) (TriggeredSeconds :type Float%20%28double-precision%29) (InputAction :type Input%20Action%20Object%20Reference :default "/Game/Inputs/IA_Mirar.IA_Mirar"))
  ;[0.15 0.15 0.15 0.5] Camara
  (Pawn|Input|AddControllerYawInput (.x ActionValue))
  (Pawn|Input|AddControllerPitchInput (.y ActionValue)))

(event Input|EnhancedActionEvents|EnhancedInputActionIA_boost
  (params (ActionValue :type Boolean) (ElapsedSeconds :type Float%20%28double-precision%29) (TriggeredSeconds :type Float%20%28double-precision%29) (InputAction :type Input%20Action%20Object%20Reference :default "/Game/Inputs/IA_boost.IA_boost"))
  ;[0.15 0.15 0.15 0.5] Boost
  (:Started
    (Utilities|FlowControl|DoOnce false :!label _label
      (:Completed
        (Development|PrintString "Boost activado " true true "(R=0.092374,G=0.120601,B=1.000000,A=1.000000)")
        (Variables|Default|SetIsBoosting true)
        (Variables|/Script/Engine.CharacterMovementComponent|SetMaxWalkSpeed (Variables|Character|GetCharacterMovement) (Variables|Default|GetBoostSpeed))
        (Utilities|FlowControl|Delay 1e+01)
        (Variables|/Script/Engine.CharacterMovementComponent|SetMaxWalkSpeed (Variables|Character|GetCharacterMovement) (Variables|Default|GetNormalSpeed))
        (Variables|Default|SetIsBoosting true))))
  (:Completed
    (Utilities|FlowControl|Delay 1e+01)
    (goto _label Reset)))

(event Input|EnhancedActionEvents|EnhancedInputActionIA_Dash
  (params (ActionValue :type Boolean) (ElapsedSeconds :type Float%20%28double-precision%29) (TriggeredSeconds :type Float%20%28double-precision%29) (InputAction :type Input%20Action%20Object%20Reference :default "/Game/Inputs/IA_Dash.IA_Dash"))
  (bind _returnvalue (Transformation|GetVelocity))
  (bind _returnvalue_2 (* _returnvalue 3.0))
  ;[0.15 0.15 0.15 0.5] DASH
  (:Started
    (Utilities|FlowControl|DoOnce false :!label _label
      (:Completed
        (Character|LaunchCharacter (Math|Vector|MakeVector (.x _returnvalue_2) (.y _returnvalue_2) 1e+02) false false))))
  (:Completed
    (Utilities|FlowControl|Delay 0.0)
    (goto _label Reset)))

(event EventBeginPlay
  (|CallParentFunction)
  (bind _asplayer_controller (Utilities|Casting|CastToPlayerController (Pawn|GetController)))
  (Utilities|IsValid (PlayerController|LocalPlayerSubsystems|GetEnhancedInputLocalPlayerSubsystem _asplayer_controller)
    (:Is%20Valid
      (Input|AddMappingContext (PlayerController|LocalPlayerSubsystems|GetEnhancedInputLocalPlayerSubsystem _asplayer_controller) "/Game/Inputs/IMC_Custom.IMC_Custom" 0 "(bIgnoreAllPressedKeysUntilRelease=True,bForceImmediately=False,bNotifyUserSettings=False)"))))

(event EventTick
  (params (DeltaSeconds :type Float%20%28single-precision%29))
  ;[0.15 0.15 0.15 0.5] Set target lock Rotation
  (Variables|Default|GetHit_Target
    (:then
      (Pawn|SetControlRotation (Pawn|GetController) (Math|Rotator|FindLookatRotation (Transformation|GetActorLocation) (Transformation|GetActorLocation (Variables|Default|GetHit_Target)))))
    (:else)))

(event Input|KeyboardEvents|Tab
  (params (Key :type Key%20Structure :default "None"))
  (bind _returnvalue (Transformation|GetActorLocation))
  ;[0.15 0.15 0.15 0.5] TARGET LOOK
  (:Pressed
    (Utilities|FlowControl|FlipFlop
      (:A
        (bind (_outhit _returnvalue_2) (Collision|SphereTraceForObjects _returnvalue (+ _returnvalue (* (Math|Vector|GetForwardVector (Transformation|GetWorldRotation (Variables|Default|GetCamera))) 500)) 125.0 (Utilities|Array|MakeArray "ObjectTypeQuery3") false 0 "ForDuration"))
        (if _returnvalue_2
          (Variables|Default|SetHit_Target (.HitActor (Collision|BreakHitResult _outhit)))))
      (:B
        (Variables|Default|SetHit_Target 0)))))

(fn ConstructionScript
  (|CallParentFunction))